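; Base quest Blueprint for the turn-based RPG template that restores a quest's state from the explore-mode hero's quest records.
; Load looks up its own class in the hero's active quest data, calling Activate with the saved step when Active, or Completed when Ready to Deliver.
; Quests found only in completed quest data also call Completed.
; Activate and Completed are empty hooks for child Blueprints, and GetSteps defaults to a single step.
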(event Custom|Load
  (bind _returnvalue (Game|Player|GetPlayerPawn 0))
  (bind _self self)
  (bind _returnvalue_2 (Utilities|GetClass _self))
  (bind _asbp_explore_hero_base (Utilities|Casting|CastToBP_ExploreHeroBase _returnvalue))
  (bind _activequestdata (Variables|/Game/TurnBasedStrategyRPGTemplate/Blueprints/Heroes/Explore/BP_ExploreHeroBase.BP_ExploreHeroBase_C|GetactiveQuestData _asbp_explore_hero_base))
  (bind (_value _returnvalue_3) (Utilities|Map|Find _activequestdata _returnvalue_2))
  ;[1 1 1] Activate quest
  (if _returnvalue_3
    (bind _queststatus (Default|GetQuestStatus _asbp_explore_hero_base (Utilities|GetClass self)))
    (switch Utilities|FlowControl|Switch|SwitchonE_QuestStatus _queststatus
      (:NewEnumerator1
        (CallFunction|Activate (.currentStep (Utilities|Struct|BreakS_QuestStepData _value))))
      (:NewEnumerator2
        (CallFunction|Completed :!label _label)))
    (elif (.ReturnValue (Utilities|Map|Find (Variables|/Game/TurnBasedStrategyRPGTemplate/Blueprints/Heroes/Explore/BP_ExploreHeroBase.BP_ExploreHeroBase_C|GetcompletedQuestData _asbp_explore_hero_base) _returnvalue_2))
      (goto _label))))

(event Custom|Activate
  (params (currentStep :type Integer))
  ;[1 1 1] Override on children BP
)

(event Custom|Completed
  ;[1 1 1] Override on children BP
)

(fn ConstructionScript)

(fn GetSteps
  ;[1 1 1] Return number of steps to completed this quest
  (return 1))