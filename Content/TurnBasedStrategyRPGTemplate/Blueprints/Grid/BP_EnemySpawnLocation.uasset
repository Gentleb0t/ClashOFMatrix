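; Editor-placed marker that designates an enemy spawn location on the tactical grid.
; Its construction script finds slots overlapping its Box, snaps its Sphere to an empty, non-inner slot, attaches to that Grid and registers in EnemySpawnLocations.
; RemoveSpawnLocation clears the slot reference and grid entry, keeping the list in sync as the marker moves or is destroyed.
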(event Custom|RemoveSpawnLocation
  (params (actor :type Actor%20Object%20Reference))
  ;[1 1 1] Remove enemy spawn location on grid
  (Utilities|IsValid (Variables|Default|Getslot)
    (:Is%20Valid
      (Utilities|Array|RemoveItem (Variables|/Game/TurnBasedStrategyRPGTemplate/Blueprints/Grid/BP_Grid.BP_Grid_C|GetenemySpawnLocations (Variables|/Game/TurnBasedStrategyRPGTemplate/Blueprints/Grid/Slots/BP_SlotBase.BP_SlotBase_C|Getgrid (Variables|Default|Getslot))) self)
      (Variables|Default|Setslot 0))))

(fn ConstructionScript
  ;[1 1 1] Snap on grid
  (|CallParentFunction)
  (Game|BindEventtoOnDestroyed (EventDispatchers|CreateEvent :!event Custom|RemoveSpawnLocation))
  (CallFunction|RemoveSpawnLocation)
  (bind _outactors (Collision|ComponentOverlapActors (Variables|Default|GetBox) (Transformation|GetWorldTransform (Variables|Default|GetBox)) (Utilities|Array|MakeArray "ObjectTypeQuery2") "/Game/TurnBasedStrategyRPGTemplate/Blueprints/Grid/Slots/BP_Slot.BP_Slot_C"))
  (if (> (Utilities|Array|Length _outactors) 0)
    (for _array_element _outactors
      (bind _asbp_slot (Utilities|Casting|CastToBP_Slot _array_element))
      (bind _output_get (LocalVariables|SetcurrentSlot _asbp_slot))
      (if (and (Default|IsEmpty _output_get) (not (Variables|/Game/TurnBasedStrategyRPGTemplate/Blueprints/Grid/Slots/BP_Slot.BP_Slot_C|GetisInnerSlot _output_get)))
        (Utilities|IsValid (Variables|Default|Getslot)
          (:Is%20Valid
            (CallFunction|RemoveSpawnLocation))
          (:Is%20Not%20Valid
            _))
        (Transformation|SetWorldLocation (Variables|Default|GetSphere) (Transformation|GetActorLocation (LocalVariables|GetcurrentSlot)) false true)
        (Transformation|AttachActorToActor (Variables|/Game/TurnBasedStrategyRPGTemplate/Blueprints/Grid/Slots/BP_SlotBase.BP_SlotBase_C|Getgrid (LocalVariables|GetcurrentSlot)) "None" "KeepWorld" "KeepWorld" "KeepWorld" true)
        (Utilities|Array|AddUnique (Variables|/Game/TurnBasedStrategyRPGTemplate/Blueprints/Grid/BP_Grid.BP_Grid_C|GetenemySpawnLocations (Variables|/Game/TurnBasedStrategyRPGTemplate/Blueprints/Grid/Slots/BP_SlotBase.BP_SlotBase_C|Getgrid (LocalVariables|GetcurrentSlot))) self)
        (Variables|Default|Setslot (LocalVariables|GetcurrentSlot))))
    (else
      (CallFunction|RemoveSpawnLocation))))