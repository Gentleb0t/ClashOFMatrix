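; BP_AllyTargetSpellBase is the base Blueprint for turn-based strategy spells that target allied units.
; Enabling or disabling the spell notifies the BattleController's Grid to switch ally-target mode.
; A target slot is stored on the spell, and GetSpellSlots casts its contained unit to BP_CharacterBase.
; That unit is added uniquely to CurrentAllies, which is returned without being cleared here.
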(event EventOnSpellEnabled
  ;[1 1 1] Enable / disable ally target spell
  (Default|OnAllyTargetSpellEnabled (Variables|/Game/TurnBasedStrategyRPGTemplate/Blueprints/Core/BP_BattleController.BP_BattleController_C|Getgrid (Variables|Default|GetbattleController))))

(event EventOnSpellDisabled
  ;[1 1 1] Enable / disable ally target spell
  (Default|OnAllyTargetSpellDisabled (Variables|/Game/TurnBasedStrategyRPGTemplate/Blueprints/Core/BP_BattleController.BP_BattleController_C|Getgrid (Variables|Default|GetbattleController))))

(event EventSetTargetSlot
  (params (slot :type BP%20Slot%20Base%20Object%20Reference))
  ;[1 1 1] Set target slot for the spell
  (Variables|Default|SettargetSlot slot))

(fn ConstructionScript
  (|CallParentFunction))

(fn GetSpellSlots
  ;[1 1 1] Return allies in target slot
  (Utilities|IsValid (Variables|Default|GettargetSlot)
    (:Is%20Valid
      (Utilities|Array|AddUnique (LocalVariables|GetcurrentAllies) (.AsBP%20Character%20Base (Utilities|Casting|CastToBP_CharacterBase (Variables|/Game/TurnBasedStrategyRPGTemplate/Blueprints/Grid/Slots/BP_SlotBase.BP_SlotBase_C|GetcontainedUnit (Variables|Default|GettargetSlot)))))
      (return 0 0 (LocalVariables|GetcurrentAllies) 0))
    (:Is%20Not%20Valid
      (return 0 0 (LocalVariables|GetcurrentAllies) 0))))