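; BP_ResurrectionSpell is an ally-target hero spell that resurrects fallen units in allied stacks.
; On use, it runs the parent spell logic, then converts a health pool scaled from the hero's power stat into whole units using each target's max health.
; It passes that count to Resurrect on every ally it receives, then ends the spell.
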(event EventOnSpellUsed
  (params (emptySlots :type Array%20of%20BP%20Slot%20Base%20Object%20References) (allies :type Array%20of%20BP%20Character%20Base%20Object%20References) (enemies :type Array%20of%20BP%20Character%20Base%20Object%20References))
  ;[1 1 1] Resurrect (hero's stats power * 2) + 25 health worth of dying stack
  (|CallParentFunction emptySlots allies enemies)
  (for _array_element allies
    (bind _output_get (Variables|Default|SettargetCharacter _array_element))
    (Default|Resurrect _output_get (.ReturnValue (Math|Float|Division(WholeandRemainder) (Math|Conversions|ToFloat(Integer) (+ (* (.power (Variables|/Game/TurnBasedStrategyRPGTemplate/Blueprints/Heroes/Battle/BP_BattleHeroBase.BP_BattleHeroBase_C|GetheroStats (Variables|Default|Gethero))) 2) 25)) (Math|Conversions|ToFloat(Integer) (.maxhealth (Variables|/Game/TurnBasedStrategyRPGTemplate/Blueprints/Units/Characters/BP_CharacterBase.BP_CharacterBase_C|GetmainStats (Variables|Default|GettargetCharacter))))))))
  (CallFunction|EndSpell))

(fn ConstructionScript
  (|CallParentFunction))